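; BP_Enemy_2 is a melee enemy tied to BP_Boss that heals the player and increments the boss's TpBack when killed.
; PawnSensing triggers an AIMoveTo chase, then a montage attack whose timed delays open a damage window for the Box overlap.
; Capsule overlaps subtract player Damage from AiHealth, with death checked on Tick.
; Until it sees the player it stands still, relocating randomly once when boss health is low.
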(event `self.ReceiveTick`
  (params (DeltaSeconds :type "Float (single-precision)"))
  ;[1 1 1] Enemy movement and attack
  (if (`self.IsSeeingPlayer?`)
    (if (<= (`self.Ai_Health`) 0.0)
      (bind _asbp_player (cast `/Game/Blueprint/Blueprints/BP_Player` (`GameplayStatics.GetPlayerCharacter` 0)))
      (set `/Game/Blueprint/Blueprints/BP_Player.Player_Health` (+ (`/Game/Blueprint/Blueprints/BP_Player.Player_Health` _asbp_player) 0.1) _asbp_player)
      (`self.K2_DestroyActor`)
      (bind _outactors (`GameplayStatics.GetAllActorsOfClass` "/Game/Blueprint/Blueprints/BP_Boss.BP_Boss_C"))
      (bind _output (`|GetArrayItem` _outactors))
      (set `/Game/Blueprint/Blueprints/BP_Boss.tp_back` (+ (`/Game/Blueprint/Blueprints/BP_Boss.tp_back` _output) 1) _output))
    (else
      (`MovementComponent.StopMovementImmediately` (`self.CharacterMovement`))
      (bind _outactors_2 (`GameplayStatics.GetAllActorsOfClass` "/Game/Blueprint/Blueprints/BP_Boss.BP_Boss_C"))
      (if (<= (`/Game/Blueprint/Blueprints/BP_Boss.BossHealth` (`|GetArrayItem` _outactors_2)) 4.0)
        (`/Engine/EditorBlueprintResources/StandardMacros.DoOnce` false
          (:`Completed`
            (`self.K2_SetActorTransform` (`KismetMathLibrary.MakeTransform` (`KismetMathLibrary.MakeVector` (+ 1950.0 (`KismetMathLibrary.RandomFloatInRange` -1000.0 1000.0)) (+ 0.0 (`KismetMathLibrary.RandomFloatInRange` -1000.0 1000.0)) 110.0)))))))))

(event `self.PawnSensing.OnSeePawn`
  (params (Pawn :type "Pawn Object Reference"))
  ;[1 1 1] Enemy movement and attack
  (set `self.IsSeeingPlayer?` true)
  (`self.FollowPlayer`))

(event `FollowPlayer`
  ;[1 1 1] Enemy movement and attack
  (if (`self.IsSeeingPlayer?`)
    (if (`self.Follow`)
      (`|AIMoveTo` self (0.0 0.0 0.0) (`GameplayStatics.GetPlayerCharacter` 0) 70.0
        (:`OnSuccess`
          (if (`self.CanAttack?`)
            (set `self.CanAttack?` false)
            (set `self.Follow` false)
            (`self.Face`)
            (bind _returnvalue (`self.PlayAnimMontage` "/Game/Animations/Enemy/Movement/Standing_Melee_Attack_Downward_Montage.Standing_Melee_Attack_Downward_Montage"))
            (`KismetSystemLibrary.Delay` 0.38)
            (set `self.Ai_Damage` 0.1)
            (`KismetSystemLibrary.Delay` 1.0)
            (set `self.Ai_Damage` 0.0)
            (`KismetSystemLibrary.Delay` (- _returnvalue 1.16))
            (set `self.CanAttack?` true)
            (set `self.Follow` true)))))
    (else
      (set `self.IsSeeingPlayer?` false))))

(event `self.Box.OnComponentBeginOverlap`
  (params (OverlappedComponent :type "PrimitiveComponent Object Reference") (OtherActor :type "Actor Object Reference") (OtherComp :type "PrimitiveComponent Object Reference") (OtherBodyIndex :type Integer) (bFromSweep :type Boolean) (SweepResult :type "HitResult Structure (by ref)"))
  ;[1 1 1] Enemy movement and attack
  (`KismetSystemLibrary.Delay` 0.5)
  (bind _asbp_player (cast `/Game/Blueprint/Blueprints/BP_Player` OtherActor))
  (set `/Game/Blueprint/Blueprints/BP_Player.Player_Health` (- (`/Game/Blueprint/Blueprints/BP_Player.Player_Health` _asbp_player) (`self.Ai_Damage`)) _asbp_player))

(event `self.CapsuleComponent.OnComponentBeginOverlap`
  (params (OverlappedComponent :type "PrimitiveComponent Object Reference") (OtherActor :type "Actor Object Reference") (OtherComp :type "PrimitiveComponent Object Reference") (OtherBodyIndex :type Integer) (bFromSweep :type Boolean) (SweepResult :type "HitResult Structure (by ref)"))
  (`KismetSystemLibrary.Delay` 0.2)
  (bind _asbp_player (cast `/Game/Blueprint/Blueprints/BP_Player` OtherActor))
  (set `self.Ai_Health` (- (`self.Ai_Health`) (`/Game/Blueprint/Blueprints/BP_Player.Damage` _asbp_player)))
  (if (not (`/Game/Blueprint/Blueprints/BP_Player.MovementOn` _asbp_player))
    (`self.PlayAnimMontage` "/Game/Animations/Enemy/Movement/Getting_Hit_Montage.Getting_Hit_Montage")))

(event `Face`
  ;[1 1 1] Face player
  (bind _asbp_player (cast `/Game/Blueprint/Blueprints/BP_Player` (`GameplayStatics.GetPlayerCharacter` 0)))
  (bind _output_get (set `self.PlayerRef` _asbp_player))
  (bind (_returnvalue_roll _returnvalue_pitch _returnvalue_yaw) (`KismetMathLibrary.BreakRotator` (`KismetMathLibrary.RInterpTo` (`self.K2_GetActorRotation`) (`KismetMathLibrary.FindLookAtRotation` (`self.K2_GetActorLocation`) (`self.K2_GetActorLocation` _output_get)) (`GameplayStatics.GetWorldDeltaSeconds`) 70.0)))
  (`self.K2_SetActorRotation` (`KismetMathLibrary.MakeRotator` 0.0 0.0 _returnvalue_yaw)))

(fn `UserConstructionScript`)