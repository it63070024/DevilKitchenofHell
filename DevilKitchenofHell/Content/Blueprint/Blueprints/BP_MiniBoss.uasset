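; Mini-boss enemy that roars on first spotting the player through PawnSensing, then chases with AIMoveTo and health widget.
; On reaching the player it plays one of three random melee montages, using delays to set the damage its hitbox overlap applies.
; Its own health lives on BP_Player, drops by the player's Damage on capsule overlap, and triggers death from Tick at zero.
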(event `self.ReceiveTick`
  (params (DeltaSeconds :type "Float (single-precision)"))
  ;[1 1 1] Enemy movement and attack
  (if (not (`self.IsSeeingPlayer?`))
    (`MovementComponent.StopMovementImmediately` (`self.CharacterMovement`)))
  (bind _asbp_player (cast `/Game/Blueprint/Blueprints/BP_Player` (`GameplayStatics.GetPlayerCharacter` 0)))
  (if (<= (`/Game/Blueprint/Blueprints/BP_Player.MiniBossHealth` _asbp_player) 0.0)
    (`/Engine/EditorBlueprintResources/StandardMacros.DoOnce` false
      (:`Completed`
        (set `self.Died?` true)
        (`self.PlayAnimMontage` "/Game/Animations/MiniBoss/WalkMovement/Dying_miniboss_Montage.Dying_miniboss_Montage")
        (`SkeletalMeshComponent.PlayAnimation` (`self.Mesh`) "/Game/Animations/MiniBoss/WalkMovement/MiniBoss_Died.MiniBoss_Died" true)))))

(event `self.PawnSensing.OnSeePawn`
  (params (Pawn :type "Pawn Object Reference"))
  (if (`self.first_time`)
    (`/Engine/EditorBlueprintResources/StandardMacros.DoOnce` false
      (:`Completed`
        (bind _returnvalue (`self.PlayAnimMontage` "/Game/Animations/MiniBoss/AttackMovement/Mutant_Roaring_Montage.Mutant_Roaring_Montage"))
        ;[1 1 1] Enemy movement and attack
        (`KismetSystemLibrary.Delay` _returnvalue)
        (set `self.first_time` false)))
    (elif (not (`self.Died?`))
      (set `self.IsSeeingPlayer?` true)
      (`self.FollowPlayer`))))

(event `FollowPlayer`
  (bind _returnvalue (`KismetMathLibrary.RandomInteger` 3))
  ;[1 1 1] Enemy movement and attack
  (if (`self.IsSeeingPlayer?`)
    (bind _returnvalue_2 (`|CreateWidget` "/Game/DevilcKitchen/Widget/MiniBossHealth_Widget.MiniBossHealth_Widget_C"))
    (`UserWidget.AddToViewport` _returnvalue_2 0)
    (if (`self.Follow`)
      (`|AIMoveTo` self (0.0 0.0 0.0) (`GameplayStatics.GetPlayerCharacter` 0) 70.0
        (:`OnSuccess`
          (if (`self.CanAttack?`)
            (set `self.CanAttack?` false)
            (set `self.Follow` false)
            (if (== _returnvalue 0)
              (bind _returnvalue_3 (`self.PlayAnimMontage` "/Game/Animations/MiniBoss/AttackMovement/Standing_Taunt_Battlecry_Montage.Standing_Taunt_Battlecry_Montage"))
              (`KismetSystemLibrary.Delay` _returnvalue_3)
              (`self.Face`)
              (bind _returnvalue_4 (`self.PlayAnimMontage` "/Game/Animations/MiniBoss/AttackMovement/Standing_Melee_Combo_Attack_Ver__2_Montage.Standing_Melee_Combo_Attack_Ver__2_Montage"))
              (`KismetSystemLibrary.Delay` 0.6)
              (set `self.HowMuchDamage?` 0.15)
              (`KismetSystemLibrary.Delay` (- _returnvalue_4 0.6))
              (elif (== _returnvalue 1)
                (`self.Face`)
                (bind _returnvalue_5 (`self.PlayAnimMontage` "/Game/Animations/MiniBoss/AttackMovement/Stable_Sword_Inward_Slash_Montage.Stable_Sword_Inward_Slash_Montage"))
                (`KismetSystemLibrary.Delay` 1.15)
                (set `self.HowMuchDamage?` 0.25)
                (`KismetSystemLibrary.Delay` (- _returnvalue_5 1.15))
                (else
                  (`self.Face`)
                  (bind _returnvalue_6 (`self.PlayAnimMontage` "/Game/Animations/MiniBoss/AttackMovement/Standing_Melee_Attack_360_Low_Montage.Standing_Melee_Attack_360_Low_Montage"))
                  (`KismetSystemLibrary.Delay` 0.83)
                  (set `self.HowMuchDamage?` 0.2)
                  (`KismetSystemLibrary.Delay` (- _returnvalue_6 0.83)))))
            (set `self.CanAttack?` true)
            (set `self.Follow` true)
            (set `self.HowMuchDamage?` 0.0)))))
    (else
      (set `self.IsSeeingPlayer?` false))))

(event `self.ReceiveBeginPlay`
  (set `self.MinibossLoc` (`self.GetTransform`)))

(event `self.Box.OnComponentBeginOverlap`
  (params (OverlappedComponent :type "PrimitiveComponent Object Reference") (OtherActor :type "Actor Object Reference") (OtherComp :type "PrimitiveComponent Object Reference") (OtherBodyIndex :type Integer) (bFromSweep :type Boolean) (SweepResult :type "HitResult Structure (by ref)"))
  ;[1 1 1] Enemy movement and attack
  (`KismetSystemLibrary.Delay` 0.2)
  (bind _asbp_player (cast `/Game/Blueprint/Blueprints/BP_Player` OtherActor))
  (set `/Game/Blueprint/Blueprints/BP_Player.Player_Health` (- (`/Game/Blueprint/Blueprints/BP_Player.Player_Health` _asbp_player) (`self.HowMuchDamage?`)) _asbp_player)
  (`GameplayStatics.PlaySound2D` "/Game/Sound/bossSlash.bossSlash" 1.0 1.0 0.0 null null))

(event `self.CapsuleComponent.OnComponentBeginOverlap`
  (params (OverlappedComponent :type "PrimitiveComponent Object Reference") (OtherActor :type "Actor Object Reference") (OtherComp :type "PrimitiveComponent Object Reference") (OtherBodyIndex :type Integer) (bFromSweep :type Boolean) (SweepResult :type "HitResult Structure (by ref)"))
  (`KismetSystemLibrary.Delay` 0.2)
  (bind _asbp_player (cast `/Game/Blueprint/Blueprints/BP_Player` OtherActor))
  (set `/Game/Blueprint/Blueprints/BP_Player.MiniBossHealth` (- (`/Game/Blueprint/Blueprints/BP_Player.MiniBossHealth` _asbp_player) (`/Game/Blueprint/Blueprints/BP_Player.Damage` _asbp_player)) _asbp_player))

(event `Face`
  ;[1 1 1] Face player
  (bind _asbp_player (cast `/Game/Blueprint/Blueprints/BP_Player` (`GameplayStatics.GetPlayerCharacter` 0)))
  (bind _output_get (set `self.PlayerRef` _asbp_player))
  (bind (_returnvalue_roll _returnvalue_pitch _returnvalue_yaw) (`KismetMathLibrary.BreakRotator` (`KismetMathLibrary.RInterpTo` (`self.K2_GetActorRotation`) (`KismetMathLibrary.FindLookAtRotation` (`self.K2_GetActorLocation`) (`self.K2_GetActorLocation` _output_get)) (`GameplayStatics.GetWorldDeltaSeconds`) 50.0)))
  (`self.K2_SetActorRotation` (`KismetMathLibrary.MakeRotator` 0.0 0.0 _returnvalue_yaw)))

(fn `UserConstructionScript`)