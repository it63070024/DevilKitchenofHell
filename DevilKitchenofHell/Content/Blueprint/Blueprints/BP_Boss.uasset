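; Boss enemy that roars when it first senses the player, then turns to face and chase them with AIMoveTo.
; In range, it randomly slashes, stabs or chains a slash into a blink jump attack, timing delays to pulse two damage hitboxes.
; Capsule overlaps subtract player damage from boss health.
; At low health it teleports away until TpBack reaches three, returns for the next phase, and plays a death montage at zero.
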(event `ChangeCollision`
  (`PrimitiveComponent.SetCollisionEnabled` (`self.Box1`) "QueryOnly")
  (`PrimitiveComponent.SetCollisionEnabled` (`self.Box`) "QueryOnly")
  (`KismetSystemLibrary.Delay` 0.05)
  (`PrimitiveComponent.SetCollisionEnabled` (`self.Box1`) "NoCollision")
  (`PrimitiveComponent.SetCollisionEnabled` (`self.Box`) "NoCollision"))

(event `ChangeToPhy`
  (`PrimitiveComponent.SetCollisionEnabled` (`self.Box1`) "QueryAndPhysics")
  (`PrimitiveComponent.SetCollisionEnabled` (`self.Box`) "QueryAndPhysics")
  (`KismetSystemLibrary.Delay` 0.05)
  (`PrimitiveComponent.SetCollisionEnabled` (`self.Box1`) "NoCollision")
  (`PrimitiveComponent.SetCollisionEnabled` (`self.Box`) "NoCollision"))

(event `self.ReceiveTick`
  (params (DeltaSeconds :type "Float (single-precision)"))
  ;[1 1 1] Enemy movement and attack
  (if (`self.IsSeeingPlayer?`)
    (`self.Face`))
  (if (and (<= (`self.BossHealth`) 4.0) (not (`self.Phase1Complete`)))
    (`self.K2_SetActorTransform` (`KismetMathLibrary.MakeTransform` (3000.0 12200.0 688.0)))
    (if (== (`self.tp_back`) 3)
      (`self.K2_SetActorTransform` (`KismetMathLibrary.MakeTransform` (1950.0 0.0 110.0)))
      (set `self.Phase1Complete` true))
    (elif (<= (`self.BossHealth`) 0.0)
      (`/Engine/EditorBlueprintResources/StandardMacros.DoOnce` false
        (:`Completed`
          (set `self.Died?` true)
          (`self.PlayAnimMontage` "/Game/Animations/MiniBoss/WalkMovement/Dying_miniboss_Montage.Dying_miniboss_Montage"))))))

(event `self.PawnSensing.OnSeePawn`
  (params (Pawn :type "Pawn Object Reference"))
  (if (`self.first_time`)
    (`/Engine/EditorBlueprintResources/StandardMacros.DoOnce` false
      (:`Completed`
        (bind _returnvalue (`self.PlayAnimMontage` "/Game/Animations/MiniBoss/AttackMovement/Mutant_Roaring_Montage.Mutant_Roaring_Montage"))
        ;[1 1 1] Enemy movement and attack
        (`KismetSystemLibrary.Delay` _returnvalue)
        (set `self.first_time` false)))
    (elif (not (`self.Died?`))
      (set `self.IsSeeingPlayer?` true)
      (`self.FollowPlayer`))))

(event `FollowPlayer`
  (bind _returnvalue (`KismetMathLibrary.RandomInteger` 3))
  (bind (_returnvalue_roll _returnvalue_pitch _returnvalue_yaw) (`KismetMathLibrary.BreakRotator` (`self.K2_GetActorRotation`)))
  ;[1 1 1] Enemy movement and attack
  (if (`self.IsSeeingPlayer?`)
    (bind _returnvalue_2 (`|CreateWidget` "/Game/DevilcKitchen/Widget/BossHealth_Widget.BossHealth_Widget_C"))
    (`UserWidget.AddToViewport` _returnvalue_2 0)
    (if (`self.Follow`)
      (`|AIMoveTo` self (0.0 0.0 0.0) (`GameplayStatics.GetPlayerCharacter` 0) 70.0
        (:`OnSuccess`
          (if (`self.CanAttack?`)
            (set `self.CanAttack?` false)
            (set `self.Follow` false)
            (if (== _returnvalue 0)
              (bind _returnvalue_3 (`self.PlayAnimMontage` "/Game/Animations/Boss/CombatAnim/Slash.Slash"))
              (set `self.HowMuchDamage?` 0.05)
              (`self.K2_AddActorLocalOffset` (-50.0 0.0 0.0))
              (`KismetSystemLibrary.Delay` 0.5)
              (`self.ChangeCollision`)
              (`KismetSystemLibrary.Delay` 1.0)
              (`self.ChangeCollision`)
              (`KismetSystemLibrary.Delay` 0.34)
              (`self.ChangeCollision`)
              (`KismetSystemLibrary.Delay` (- _returnvalue_3 1.84))
              (bind _asbp_player (cast `/Game/Blueprint/Blueprints/BP_Player` (`GameplayStatics.GetPlayerCharacter` 0)))
              (`NiagaraFunctionLibrary.SpawnSystemAtLocation` "/Game/BlinkAndDashVFX/VFX_Niagara/NS_Blink_DarkMagic.NS_Blink_DarkMagic" (`self.K2_GetActorLocation`))
              (bind (_returnvalue_x _returnvalue_y) (`KismetMathLibrary.BreakVector` (`self.K2_GetActorLocation` _asbp_player)))
              (`self.K2_SetActorLocation` (`KismetMathLibrary.MakeVector` (- _returnvalue_x 200.0) _returnvalue_y 186.0))
              (`NiagaraFunctionLibrary.SpawnSystemAtLocation` "/Game/BlinkAndDashVFX/VFX_Niagara/NS_Blink_DarkMagic.NS_Blink_DarkMagic" (`self.K2_GetActorLocation`) (struct) (0.5 0.5 0.5))
              (`KismetSystemLibrary.Delay` 0.1)
              (set `self.CanFacePlayer?` false)
              (`self.K2_SetActorRotation` (`KismetMathLibrary.MakeRotator` 0.0 0.0 (+ _returnvalue_yaw 1.0)))
              (bind _returnvalue_4 (`self.PlayAnimMontage` "/Game/Animations/Boss/CombatAnim/Jump_Attack_Montage.Jump_Attack_Montage"))
              (set `self.HowMuchDamage?` 0.25)
              (`KismetSystemLibrary.Delay` 0.9)
              (`self.ChangeCollision`)
              (`KismetSystemLibrary.Delay` (- _returnvalue_4 0.9))
              (set `self.CanFacePlayer?` true)
              (elif (== _returnvalue 1)
                (bind _returnvalue_5 (`self.PlayAnimMontage` "/Game/Animations/Boss/CombatAnim/Slash.Slash"))
                (set `self.HowMuchDamage?` 0.05)
                (`self.K2_AddActorLocalOffset` (-50.0 0.0 0.0))
                (`KismetSystemLibrary.Delay` 0.5)
                (`self.ChangeCollision`)
                (`KismetSystemLibrary.Delay` 1.0)
                (`self.ChangeCollision`)
                (`KismetSystemLibrary.Delay` 0.34)
                (`self.ChangeCollision`)
                (`KismetSystemLibrary.Delay` (- _returnvalue_5 1.84))
                (else
                  (bind _returnvalue_6 (`self.PlayAnimMontage` "/Game/Animations/Boss/CombatAnim/stab.stab"))
                  (set `self.HowMuchDamage?` 0.05)
                  (`KismetSystemLibrary.Delay` 0.23)
                  (`self.ChangeCollision`)
                  (`KismetSystemLibrary.Delay` 0.24)
                  (`self.ChangeCollision`)
                  (`KismetSystemLibrary.Delay` 0.25)
                  (`self.ChangeCollision`)
                  (`KismetSystemLibrary.Delay` 0.57)
                  (`self.ChangeCollision`)
                  (`KismetSystemLibrary.Delay` 0.27)
                  (`KismetSystemLibrary.Delay` (- _returnvalue_6 156.0)))))
            (set `self.CanAttack?` true)
            (set `self.Follow` true)
            (set `self.HowMuchDamage?` 0.0)))))
    (else
      (set `self.IsSeeingPlayer?` false))))

(event `self.ReceiveBeginPlay`)

(event `self.Box.OnComponentBeginOverlap`
  (params (OverlappedComponent :type "PrimitiveComponent Object Reference") (OtherActor :type "Actor Object Reference") (OtherComp :type "PrimitiveComponent Object Reference") (OtherBodyIndex :type Integer) (bFromSweep :type Boolean) (SweepResult :type "HitResult Structure (by ref)"))
  ;[1 1 1] Enemy movement and attack
  (`KismetSystemLibrary.Delay` 0.2)
  (bind _asbp_player (cast `/Game/Blueprint/Blueprints/BP_Player` OtherActor))
  (set `/Game/Blueprint/Blueprints/BP_Player.Player_Health` (- (`/Game/Blueprint/Blueprints/BP_Player.Player_Health` _asbp_player) (`self.HowMuchDamage?`)) _asbp_player)
  (`GameplayStatics.PlaySound2D` "/Game/Sound/bossSlash.bossSlash" 0.4 1.0 0.0 null null :!label _label))

(event `self.Box1.OnComponentBeginOverlap`
  (params (OverlappedComponent :type "PrimitiveComponent Object Reference") (OtherActor :type "Actor Object Reference") (OtherComp :type "PrimitiveComponent Object Reference") (OtherBodyIndex :type Integer) (bFromSweep :type Boolean) (SweepResult :type "HitResult Structure (by ref)"))
  ;[1 1 1] Enemy movement and attack
  (`KismetSystemLibrary.Delay` 0.2)
  (bind _asbp_player (cast `/Game/Blueprint/Blueprints/BP_Player` OtherActor))
  (set `/Game/Blueprint/Blueprints/BP_Player.Player_Health` (- (`/Game/Blueprint/Blueprints/BP_Player.Player_Health` _asbp_player) (`self.HowMuchDamage?`)) _asbp_player)
  (goto _label))

(event `self.CapsuleComponent.OnComponentBeginOverlap`
  (params (OverlappedComponent :type "PrimitiveComponent Object Reference") (OtherActor :type "Actor Object Reference") (OtherComp :type "PrimitiveComponent Object Reference") (OtherBodyIndex :type Integer) (bFromSweep :type Boolean) (SweepResult :type "HitResult Structure (by ref)"))
  (`KismetSystemLibrary.Delay` 0.2)
  (bind _asbp_player (cast `/Game/Blueprint/Blueprints/BP_Player` OtherActor))
  (set `self.BossHealth` (- (`self.BossHealth`) (`/Game/Blueprint/Blueprints/BP_Player.Damage` _asbp_player))))

(event `Face`
  ;[1 1 1] Face player
  (if (`self.CanFacePlayer?`)
    (bind _asbp_player (cast `/Game/Blueprint/Blueprints/BP_Player` (`GameplayStatics.GetPlayerCharacter` 0)))
    (bind _output_get (set `self.PlayerRef` _asbp_player))
    (bind (_returnvalue_roll _returnvalue_pitch _returnvalue_yaw) (`KismetMathLibrary.BreakRotator` (`KismetMathLibrary.RInterpTo` (`self.K2_GetActorRotation`) (`KismetMathLibrary.FindLookAtRotation` (`self.K2_GetActorLocation`) (`self.K2_GetActorLocation` _output_get)) (`GameplayStatics.GetWorldDeltaSeconds`) 50.0)))
    (`self.K2_SetActorRotation` (`KismetMathLibrary.MakeRotator` 0.0 0.0 _returnvalue_yaw))))

(fn `UserConstructionScript`)